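; BP_Enemy is an enemy Blueprint that provides the scale-based spawn, hit and death animations for its static mesh.
; OnSpawn, OnHit and OnDeath each play a timeline (ScaleUp, Shake or ScaleDown) that drives uniform mesh scale, then call a matching completion function.
; The hit shake restarts on every hit.
; Nodes for disabling mesh collision during animation are present but never run.
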(event EventOnHit
  ;[0 0 0] Animations
  (bind _scale (Timeline|Shake PlayFromStart)
    (:Update
      (Transformation|SetRelativeScale3D (Variables|Default|GetStaticMesh) (Math|Vector|MakeVector _scale _scale _scale)))
    (:Finished
      (Class|EnemyCharacter|OnHitAnimationCompete))))

(event EventOnSpawn
  ;[0 0 0] Animations
  (bind _scale (Timeline|Scale%20Up Play)
    (:Update
      (Transformation|SetRelativeScale3D (Variables|Default|GetStaticMesh) (Math|Vector|MakeVector _scale _scale _scale)))
    (:Finished
      (Class|EnemyCharacter|OnSpawnAnimationComplete))))

(event EventOnDeath
  ;[0 0 0] Animations
  (bind _scale (Timeline|Scale%20Down Play)
    (:Update
      (Transformation|SetRelativeScale3D (Variables|Default|GetStaticMesh) (Math|Vector|MakeVector _scale _scale _scale)))
    (:Finished
      (Class|EnemyCharacter|OnDeathAnimationComplete))))

(fn ConstructionScript)