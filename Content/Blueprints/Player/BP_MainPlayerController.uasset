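; Player controller that lets the player tune a string-based ability and shows its current stats on screen.
; Enhanced Input actions call StringAbilityComponent to upgrade or degrade, enlarge or shrink, speed up or slow down, and widen or constrict the ability.
; Each change refreshes the WBP_HUD created on BeginPlay with the component's harmonic, damage radius, amplitude and period.
; Escape quits the game.
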(event Custom|Update%20HUD
  (bind _hud (Variables|Default|GetHUD))
  (bind _stringabilitycomponent (Variables|Default|GetStringAbilityComponent))
  ;[0 0 0] HUD Updates
  (Default|UpdateHarmonicNumber _hud (Class|StringAbilityComponent|GetHarmonic _stringabilitycomponent))
  (Default|UpdateDamageRadius _hud (Class|StringAbilityComponent|GetDamageRadius _stringabilitycomponent))
  (Default|UpdateAmplitude _hud (Class|StringAbilityComponent|GetAmplitude _stringabilitycomponent))
  (Default|UpdatePeriod _hud (Class|StringAbilityComponent|GetPeriod _stringabilitycomponent)))

(event Input|EnhancedActionEvents|EnhancedInputActionIA_UpgradeAbility
  (params (ActionValue :type Boolean) (ElapsedSeconds :type Float%20%28double-precision%29) (TriggeredSeconds :type Float%20%28double-precision%29) (InputAction :type Input%20Action%20Object%20Reference :default "/Game/Input/Actions/IA_UpgradeAbility.IA_UpgradeAbility"))
  ;[0 0 0] Ability Tweaks
  (Class|StringAbilityComponent|UpgradeAbility (Variables|Default|GetStringAbilityComponent))
  (CallFunction|UpdateHUD))

(event Input|EnhancedActionEvents|EnhancedInputActionIA_DegradeAbility
  (params (ActionValue :type Boolean) (ElapsedSeconds :type Float%20%28double-precision%29) (TriggeredSeconds :type Float%20%28double-precision%29) (InputAction :type Input%20Action%20Object%20Reference :default "/Game/Input/Actions/IA_DegradeAbility.IA_DegradeAbility"))
  ;[0 0 0] Ability Tweaks
  (Class|StringAbilityComponent|DegradeAbility (Variables|Default|GetStringAbilityComponent))
  (CallFunction|UpdateHUD))

(event Input|EnhancedActionEvents|EnhancedInputActionIA_EnlargeAbility
  (params (ActionValue :type Boolean) (ElapsedSeconds :type Float%20%28double-precision%29) (TriggeredSeconds :type Float%20%28double-precision%29) (InputAction :type Input%20Action%20Object%20Reference :default "/Game/Input/Actions/IA_EnlargeAbility.IA_EnlargeAbility"))
  ;[0 0 0] Ability Tweaks
  (Class|StringAbilityComponent|EnlargeAbility (Variables|Default|GetStringAbilityComponent))
  (CallFunction|UpdateHUD))

(event Input|EnhancedActionEvents|EnhancedInputActionIA_ShrinkAbility
  (params (ActionValue :type Boolean) (ElapsedSeconds :type Float%20%28double-precision%29) (TriggeredSeconds :type Float%20%28double-precision%29) (InputAction :type Input%20Action%20Object%20Reference :default "/Game/Input/Actions/IA_ShrinkAbility.IA_ShrinkAbility"))
  ;[0 0 0] Ability Tweaks
  (Class|StringAbilityComponent|ShrinkAbility (Variables|Default|GetStringAbilityComponent))
  (CallFunction|UpdateHUD))

(event Input|EnhancedActionEvents|EnhancedInputActionIA_SpeedUpAbility
  (params (ActionValue :type Boolean) (ElapsedSeconds :type Float%20%28double-precision%29) (TriggeredSeconds :type Float%20%28double-precision%29) (InputAction :type Input%20Action%20Object%20Reference :default "/Game/Input/Actions/IA_SpeedUpAbility.IA_SpeedUpAbility"))
  ;[0 0 0] Ability Tweaks
  (Class|StringAbilityComponent|SpeedUpAbility (Variables|Default|GetStringAbilityComponent))
  (CallFunction|UpdateHUD))

(event Input|EnhancedActionEvents|EnhancedInputActionIA_SlowDownAbility
  (params (ActionValue :type Boolean) (ElapsedSeconds :type Float%20%28double-precision%29) (TriggeredSeconds :type Float%20%28double-precision%29) (InputAction :type Input%20Action%20Object%20Reference :default "/Game/Input/Actions/IA_SlowDownAbility.IA_SlowDownAbility"))
  ;[0 0 0] Ability Tweaks
  (Class|StringAbilityComponent|SlowDownAbility (Variables|Default|GetStringAbilityComponent))
  (CallFunction|UpdateHUD))

(event Input|EnhancedActionEvents|EnhancedInputActionIA_WidenAbility
  (params (ActionValue :type Boolean) (ElapsedSeconds :type Float%20%28double-precision%29) (TriggeredSeconds :type Float%20%28double-precision%29) (InputAction :type Input%20Action%20Object%20Reference :default "/Game/Input/Actions/IA_WidenAbility.IA_WidenAbility"))
  ;[0 0 0] Ability Tweaks
  (Class|StringAbilityComponent|WidenAbility (Variables|Default|GetStringAbilityComponent))
  (CallFunction|UpdateHUD))

(event Input|EnhancedActionEvents|EnhancedInputActionIA_ConstrictAbility
  (params (ActionValue :type Boolean) (ElapsedSeconds :type Float%20%28double-precision%29) (TriggeredSeconds :type Float%20%28double-precision%29) (InputAction :type Input%20Action%20Object%20Reference :default "/Game/Input/Actions/IA_ConstrictAbility.IA_ConstrictAbility"))
  ;[0 0 0] Ability Tweaks
  (Class|StringAbilityComponent|ConstrictAbility (Variables|Default|GetStringAbilityComponent))
  (CallFunction|UpdateHUD))

(event EventBeginPlay
  ;[0 0 0] Begin Play
  (bind _returnvalue (UserInterface|CreateWidget "/Game/UI/WBP_HUD.WBP_HUD_C"))
  (bind _output_get (Variables|Default|SetHUD _returnvalue))
  (UserInterface|Viewport|AddtoViewport _output_get 0)
  (CallFunction|UpdateHUD))

(event Input|KeyboardEvents|Escape
  (params (Key :type Key%20Structure :default "None"))
  ;[0 0 0] Quit Game
  (:Pressed
    (Game|QuitGame 0 "Quit" false)))

(fn ConstructionScript)